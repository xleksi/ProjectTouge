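; AI-driven car that follows an ActivePath spline, with headlights on and a random body material set at BeginPlay.
; Each Tick, ForwardBox overlaps choose the action: drive forward when clear, handbrake when blocked, or reverse when ReverseBox also overlaps.
; GetPath derives steering from the yaw toward a look-ahead point along the spline tangent, inverted when reversing.
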(event Collision|EventActorBeginOverlap
  (params (OtherActor :type Actor%20Object%20Reference)))

(event EventTick
  (params (DeltaSeconds :type Float%20%28single-precision%29))
  (|CallParentFunction DeltaSeconds)
  (if (> (Utilities|Array|Length (Collision|GetOverlappingActors (Variables|Default|GetForwardBox) 0 :!class /Script/Engine.PrimitiveComponent)) 0)
    (if (> (Utilities|Array|Length (Collision|GetOverlappingActors (Variables|Default|GetReverseBox) 0 :!class /Script/Engine.PrimitiveComponent)) 0)
      (CallFunction|MoveBackward)
      (else
        (CallFunction|Brake)))
    (else
      (CallFunction|MoveForward))))

(event EventBeginPlay
  (|CallParentFunction)
  (Variables|Default|SetRearLightsMaterial (Rendering|Material|GetMaterial (Variables|Character|GetMesh) 5))
  (CallFunction|CarrLights+MaterialPreset))

(fn ConstructionScript
  (|CallParentFunction))

(fn CarrLights+MaterialPreset
  (Rendering|SetVisibility (Variables|Default|GetHeadlightR) true true)
  (Rendering|Material|SetMaterial (Variables|Character|GetMesh) 0 (Utilities|Array|Get(acopy) (Variables|Default|GetRandomColor) (Math|Random|RandomIntegerinRange 1 4))))

(fn GetPath
  (bind _returnvalue (Transformation|GetActorLocation))
  (bind _activepath (Variables|Default|GetActivePath))
  (bind _spline (Variables|/Game/Blueprints/AI_Vehicle/BP_Path.BP_Path_C|GetSpline _activepath))
  (return (Math|Float|MapRangeClamped (.yaw (Math|Rotator|Delta(Rotator) (Math|Rotator|FindLookatRotation _returnvalue (Spline|FindLocationClosesttoWorldLocation _spline (+ (* (Math|Vector|Normalize (Class|SplineComponent|FindTangentClosesttoWorldLocation _spline _returnvalue "World")) 2e+02) _returnvalue) "World")) (Transformation|GetActorRotation))) -9e+01 9e+01 -1.0 1.0)))

(fn Brake
  (Class|ChaosVehicleMovementComponent|SetHandbrakeInput (Variables|Default|GetVehicleMovementComponent) true)
  (Class|ChaosVehicleMovementComponent|SetThrottleInput (Variables|Default|GetVehicleMovementComponent) 0.0)
  (Class|ChaosVehicleMovementComponent|SetBrakeInput (Variables|Default|GetVehicleMovementComponent) 0.0))

(fn MoveForward
  (Class|ChaosVehicleMovementComponent|SetThrottleInput (Variables|Default|GetVehicleMovementComponent) 0.5)
  (Class|ChaosVehicleMovementComponent|SetBrakeInput (Variables|Default|GetVehicleMovementComponent) 0.0)
  (Class|ChaosVehicleMovementComponent|SetHandbrakeInput (Variables|Default|GetVehicleMovementComponent) false)
  (bind _returnvalue (CallFunction|GetPath))
  (Class|ChaosVehicleMovementComponent|SetSteeringInput (Variables|Default|GetVehicleMovementComponent) (* _returnvalue 2.5)))

(fn MoveBackward
  (Class|ChaosVehicleMovementComponent|SetBrakeInput (Variables|Default|GetVehicleMovementComponent) 0.5)
  (Class|ChaosVehicleMovementComponent|SetHandbrakeInput (Variables|Default|GetVehicleMovementComponent) false)
  (bind _returnvalue (CallFunction|GetPath))
  (Class|ChaosVehicleMovementComponent|SetSteeringInput (Variables|Default|GetVehicleMovementComponent) (* _returnvalue -1.0)))
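; BP_MenuVehicle is a menu vehicle that plays a scripted intro on BeginPlay.
; It activates the reverse camera, caches a rear-light material and applies a body material from RandomColor, whose random range is pinned to one fixed index.
; After a delay, a timeline moves and pitches the headlight component, then both headlight lights become visible.
; A short delay later, it applies partial throttle through the vehicle movement component.
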(event EventBeginPlay
  (Components|Activation|SetActive (Variables|Default|GetReverseCamera) true false)
  (Variables|Default|SetRearLightsMaterial_0 (Rendering|Material|GetMaterial (Variables|Character|GetMesh) 5))
  (CallFunction|CarrLights+MaterialPreset)
  (Utilities|FlowControl|Delay 5.0)
  (bind _alpha (Timeline|Timeline_1 PlayFromStart)
    (:Update
      (Transformation|SetRelativeLocationAndRotation (Variables|Default|GetHeadlights_0) (Math|Vector|MakeVector (Math|Float|Lerp 0.0 35.0 _alpha) 0.0 (Math|Float|Lerp 0.0 -54.0 _alpha)) (Math|Rotator|MakeRotator 0.0 (Math|Float|Lerp 0.0 19.5 _alpha) 0.0) false false))
    (:Finished
      (Rendering|SetVisibility (Variables|Default|GetHeadlightR_0) true true)
      (Utilities|FlowControl|Delay 2.0)
      (Class|ChaosVehicleMovementComponent|SetThrottleInput (Variables|Default|GetVehicleMovementComponent) 0.5))))

(fn ConstructionScript
  (|CallParentFunction))

(fn CarrLights+MaterialPreset
  (Rendering|Material|SetMaterial (Variables|Character|GetMesh) 0 (Utilities|Array|Get(acopy) (Variables|Default|GetRandomColor) (Math|Random|RandomIntegerinRange 4 4))))
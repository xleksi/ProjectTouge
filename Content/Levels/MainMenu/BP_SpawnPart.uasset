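; BP_SpawnPart is a main menu level actor that turns solid behind a BP_MenuVehicle and removes itself once far from it.
; When a menu vehicle stops overlapping its Box, the Box switches to the BlockAll collision profile.
; BeginPlay stores each found BP_MenuVehicle in one variable, then rechecks the distance every second through a looping Delay, destroying the actor beyond 30000 units.
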(event OnComponentEndOverlap(Box)
  (params (OverlappedComponent :type Primitive%20Component%20Object%20Reference) (OtherActor :type Actor%20Object%20Reference) (OtherComp :type Primitive%20Component%20Object%20Reference) (OtherBodyIndex :type Integer))
  (Utilities|Casting|CastToBP_MenuVehicle OtherActor)
  (Collision|SetCollisionProfileName (Variables|Default|GetBox) "BlockAll" false :!class /Script/Engine.PrimitiveComponent))

(event EventBeginPlay
  (|CallParentFunction)
  (bind _outactors (Actor|GetAllActorsOfClass "/Game/Blueprints/AI_Vehicle/BP_MenuVehicle.BP_MenuVehicle_C"))
  (for _array_element _outactors
    (bind _output_get (Variables|Default|SetMenuVehicle _array_element))
    (if (> (Math|Vector|VectorLength (- (Transformation|GetActorLocation _output_get) (Transformation|GetActorLocation))) 3e+04) :!label _label
      (Actor|DestroyActor)
      (else
        (Utilities|FlowControl|Delay 1.0)
        (goto _label)))))

(event Collision|EventActorBeginOverlap
  (params (OtherActor :type Actor%20Object%20Reference)))

(event EventTick
  (params (DeltaSeconds :type Float%20%28single-precision%29))
  (|CallParentFunction DeltaSeconds))

(fn ConstructionScript)